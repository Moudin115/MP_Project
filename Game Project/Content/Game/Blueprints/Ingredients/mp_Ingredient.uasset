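; Base ingredient Blueprint that configures itself from the Mp_DT_Ingredient data table when play begins.
; InitIngredient scans the table rows for the first whose IngredientClass exactly matches the instance's own class and stores it as Ingredient.
; BeginPlay then applies the static mesh from that row's IngredientStack to the StaticMesh component, so each class gets its data without naming a row.
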(event EventBeginPlay
  (CallFunction|InitIngredient)
  (Components|StaticMesh|SetStaticMesh (Variables|Default|GetStaticMesh) (.StaticMesh (Utilities|Struct|Breakmp_S_IngredientStack (.IngredientStack (Utilities|Struct|Breakmp_S_Ingredient (Variables|Default|GetIngredient)))))))

(fn ConstructionScript)

(fn InitIngredient
  (bind _outrownames (DataTable|GetDataTableRowNames "/Game/Game/Datatables/mp_DT_Ingredient.mp_DT_Ingredient"))
  (for _array_element _outrownames
    (bind _returnvalue (Utilities|GetDataTableRow "/Game/Game/Datatables/mp_DT_Ingredient.mp_DT_Ingredient" _array_element)
      (:then
        (if (== (.IngredientClass (Utilities|Struct|Breakmp_S_Ingredient _returnvalue)) (Utilities|GetClass self))
          (Variables|Default|SetIngredient _returnvalue)
          (return))))))