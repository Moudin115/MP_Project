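; Character Blueprint that handles player movement along fixed world axes, independent of view direction.
; Forward/back input moves it along world X and left/right along negative Y, ignoring zero values.
; Both inputs then share a step that interpolates control rotation toward a look-at direction built from axis values, using a fixed delta time.
; The player controller for that rotation is looked up by PlayerControllerID.
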(event EventBeginPlay)

(event Input|AxisEvents|InputAxisMovingForwardBackward
  (params (AxisValue :type Float%20%28single-precision%29))
  (bind _returnvalue (Math|Vector|MakeVector 1.0 0.0 0.0))
  (bind _playercontrollerid (Variables|Default|GetPlayerControllerID))
  (bind _returnvalue_2 (Class|GameplayStatics|GetPlayerControllerfromID _playercontrollerid))
  (if (!= AxisValue 0.0)
    (Pawn|Input|AddMovementInput _returnvalue AxisValue false)
    (Pawn|SetControlRotation _returnvalue_2 (Math|Interpolation|RInterpTo (Pawn|GetControlRotation _returnvalue_2 :!class /Script/Engine.Controller) (Math|Rotator|FindLookatRotation (Math|Vector|MakeVector 0.0 0.0 0.0) (+ (* _returnvalue AxisValue) (* (Math|Vector|MakeVector 0.0 -1.0 0.0) (stale Input|AxisEvents|InputAxisMovingLeftRight AxisValue)))) 0.001 5e+01))))

(event Input|AxisEvents|InputAxisMovingLeftRight
  (params (AxisValue :type Float%20%28single-precision%29))
  (bind _returnvalue (Math|Vector|MakeVector 0.0 -1.0 0.0))
  (bind _playercontrollerid (Variables|Default|GetPlayerControllerID))
  (bind _returnvalue_2 (Class|GameplayStatics|GetPlayerControllerfromID _playercontrollerid))
  (if (!= AxisValue 0.0)
    (Pawn|Input|AddMovementInput _returnvalue AxisValue false)
    (Pawn|SetControlRotation _returnvalue_2 (Math|Interpolation|RInterpTo (Pawn|GetControlRotation _returnvalue_2 :!class /Script/Engine.Controller) (Math|Rotator|FindLookatRotation (Math|Vector|MakeVector 0.0 0.0 0.0) (+ (* (Math|Vector|MakeVector 1.0 0.0 0.0) (stale Input|AxisEvents|InputAxisMovingForwardBackward AxisValue)) (* _returnvalue AxisValue))) 0.001 5e+01))))

(fn ConstructionScript)